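; BP_RespawnZone is a trigger volume that respawns actors entering it at their own safe location.
; On box overlap, it checks for the I_Respawnable interface, gets the actor's safe location through it and passes that to the actor's respawn message.
; The construction script keeps the box's X and Y position, places it at world Z Height and scales it horizontally by Size.
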(event `self.Box.OnComponentBeginOverlap`
  (params (OverlappedComponent :type "PrimitiveComponent Object Reference") (OtherActor :type "Actor Object Reference") (OtherComp :type "PrimitiveComponent Object Reference") (OtherBodyIndex :type Integer) (bFromSweep :type Boolean) (SweepResult :type "HitResult Structure (by ref)"))
  (if (`KismetSystemLibrary.DoesImplementInterface` OtherActor "/Game/Blueprints/I_Respawnable.I_Respawnable_C")
    (bind _safelocation (message `/Game/Blueprints/I_Respawnable.GetSafeLocation` OtherActor))
    (message `/Game/Blueprints/I_Respawnable.Respawn` OtherActor _safelocation)))

(fn `UserConstructionScript`
  (bind _size (`self.Size`))
  (bind (_returnvalue_x _returnvalue_y) (`KismetMathLibrary.BreakVector` (`SceneComponent.K2_GetComponentLocation` (`self.Box`))))
  (`SceneComponent.K2_SetWorldTransform` (`self.Box`) (`KismetMathLibrary.MakeTransform` (`KismetMathLibrary.MakeVector` _returnvalue_x _returnvalue_y (`self.Height`)) (struct) (`KismetMathLibrary.MakeVector` _size _size 1.0)) false false))