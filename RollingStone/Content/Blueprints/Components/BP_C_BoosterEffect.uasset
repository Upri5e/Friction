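; BP_C_BoosterEffect is an actor component that gives the player ball a boost.
; On BeginPlay it caches the owner's first primitive component and turns on physics simulation for it.
; BoostPlayer proceeds only if that owner is a BP_PlayerBall in the first enumerator of its ball state.
; It then zeroes linear velocity and applies the given force as an acceleration change, so prior momentum and mass do not affect the boost.
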(event `self.ReceiveBeginPlay`
  (bind _output_get (set `self.PrimitiveComponent` (`|GetArrayItem` (`Actor.K2_GetComponentsByClass` (`self.GetOwner`) "/Script/Engine.PrimitiveComponent"))))
  (`PrimitiveComponent.SetSimulatePhysics` _output_get true))

(fn `Boost Player`
  (params (Force :type "Vector Structure"))
  (bind _primitivecomponent (`self.PrimitiveComponent`))
  (bind _asbp_player_ball (cast `/Game/Blueprints/Actors/BP_PlayerBall` (`self.GetOwner` _primitivecomponent)))
  (if (`|EnumEquality` (`/Game/Blueprints/Actors/BP_PlayerBall.EBallState` _asbp_player_ball) "NewEnumerator0")
    (`PrimitiveComponent.SetPhysicsLinearVelocity` _primitivecomponent (0.0 0.0 0.0) false "None")
    (`PrimitiveComponent.AddForce` _primitivecomponent (`local.Force`) "None" true)))