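; BP_C_ScoreCounter is a component that keeps a numeric score for the game.
; AddScore adds points to the stored Score and floors the result at zero, and ResetScore sets it back to zero.
; GetScore applies the same floor, writing it back to Score before returning the value.
; The event graph holds no logic, so the score changes only through function calls.
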(event `self.ReceiveTick`
  (params (DeltaSeconds :type "Float (single-precision)")))

(fn `AddScore`
  (params (Points :type "Float (double-precision)"))
  (bind _output_get (set `self.Score` (+ Points (`self.Score`))))
  (if (not (>= _output_get 0.0))
    (set `self.Score` 0.0))
  (return))

(fn `GetScore`
  (returns (TotalScore :type "Float (double-precision)"))
  (if (not (>= (`self.Score`) 0.0))
    (set `self.Score` 0.0))
  (return (`self.Score`)))

(fn `ResetScore`
  (set `self.Score` 0.0))