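; Scene component that hovers its owning actor on a spring-like force while flagged as inside a gravity portal trigger.
; BeginPlay enables physics simulation on the owner's first primitive component, and SetGravityPortalInteraction supplies the trigger state and tuning.
; Each tick it traces down its local up axis and turns compression and its rate of change into a damped suspension force, applied at the component's location.
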(event `self.ReceiveBeginPlay`
  (bind _output_get (set `self.PrimitiveComponent` (`|GetArrayItem` (`Actor.K2_GetComponentsByClass` (`self.GetOwner`) "/Script/Engine.PrimitiveComponent"))))
  (`PrimitiveComponent.SetSimulatePhysics` _output_get true))

(event `self.ReceiveTick`
  (params (DeltaSeconds :type "Float (single-precision)"))
  (bind _returnvalue (`self.K2_GetComponentLocation`))
  (bind _hoverdistance (`self.HoverDistance`))
  (if (`self.bIsInTrigger`)
    (`self.PrimitiveComponent`
      (:`then`
        (bind (_outhit _returnvalue_2) (`KismetSystemLibrary.LineTraceSingle` _returnvalue (- _returnvalue (* (`self.GetUpVector`) (`self.HoverDistance`))) "TraceTypeQuery1" false (`|MakeArray` (`self.GetOwner`)) (select `bool` (`self.bDebugRay`) :`true` "ForOneFrame" :!type "EDrawDebugTrace Enum")))
        (if _returnvalue_2
          (bind _returnvalue_3 (/ (- _hoverdistance (`.Distance` (`GameplayStatics.BreakHitResult` _outhit))) _hoverdistance))
          (bind _output_get (set `self.HoverForce` (+ (* (/ (- _returnvalue_3 (`self.PreviosCompression`)) (`GameplayStatics.GetWorldDeltaSeconds`)) (`self.Damping`)) (* _returnvalue_3 (`self.Force`)))))
          (set `self.PreviosCompression` _returnvalue_3)
          (`PrimitiveComponent.AddForceAtLocation` (`self.PrimitiveComponent`) (* (`self.GetUpVector`) _output_get) (`self.K2_GetComponentLocation`) "None")))
      (:`else`))))

(fn `SetGravityPortalInteraction`
  (params (bIsInTrigger :type Boolean) (Force :type "Float (double-precision)") (HoverDistance :type "Float (double-precision)") (Damping :type "Float (double-precision)"))
  (set `self.bIsInTrigger` bIsInTrigger)
  (set `self.Force` Force)
  (set `self.HoverDistance` HoverDistance)
  (set `self.Damping` Damping))