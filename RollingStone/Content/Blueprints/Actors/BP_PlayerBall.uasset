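; Physics-driven player ball that toggles between Smooth and Rough states, with a zoomable spring-arm camera.
; Hit surfaces' physical materials combine with ball state to set Normal, Grip or Slip, changing speed, damping and applied forces.
; A Rough ball rolls on "Walkable" walls by disabling gravity, projecting movement onto the wall plane and pushing into it while gripping.
; A looping timer saves non-falling positions as safe locations, alongside a counted respawn function.
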(event `self.ReceiveBeginPlay`
  (set `self.CanMove` true)
  (set `self.currentArmDistance` (`SpringArmComponent.TargetArmLength` (`self.SpringArm`)))
  (`self.SetMaterial`)
  (set `self.currentMovementSpeed` (`self.MaxSpeed`))
  (`SceneCaptureComponent.ShowOnlyComponent` (`self.SceneCaptureComponent2D`) (`self.Sphere`))
  (`self.SaveBallLocation`))

(event `InputAction|Swaping`
  (params (Key :type "Key Structure"))
  ;[1 0 0.01458] Switch Ball State
  (:`Pressed`
    (`/Engine/EditorBlueprintResources/StandardMacros.IncrementInt` (`self.currentMat`)
      (:`  `
        (`self.SetMaterial`)
        (if (and (`self.bIsOnWall`) (`|EnumEquality` (`self.EBallState`) "NewEnumerator0"))
          (`PrimitiveComponent.AddImpulse` (`self.Sphere`) (* (`self.DownForce`) 300.0) "None" true)
          (`self.WallRollEvent` (`self.Sphere`)))))))

(event `InputAxis|MoveRight`
  (params (AxisValue :type "Float (single-precision)"))
  ;[0 0.4235 1] Movement
  (if (`self.CanMove`)
    (`PrimitiveComponent.AddImpulse` (`self.Sphere`) (* (* AxisValue (`self.currentMovementSpeed`)) (`SceneComponent.GetRightVector` (`self.Camera`))) "None" false)))

(event `InputAxis|MoveForward`
  (params (AxisValue :type "Float (single-precision)"))
  ;[0 0.4235 1] Movement
  (if (`self.CanMove`)
    (if (not (`self.bIsOnWall`))
      (set `self.PlaneNormal` (0.0 0.0 1.0)))
    (`PrimitiveComponent.AddImpulse` (`self.Sphere`) (* (`KismetMathLibrary.ProjectVectorOnToPlane` (`SceneComponent.GetForwardVector` (`self.Camera`)) (`self.PlaneNormal`)) (* (`self.currentMovementSpeed`) AxisValue)) "None" false)))

(event `InputAxis|LookUp`
  (params (AxisValue :type "Float (single-precision)"))
  ;[0 0.4235 1] Camera Movement
  (`self.AddControllerPitchInput` AxisValue))

(event `BallStateSwitched`
  (params (BallState :type "/Game/Blueprints/Enums/E_BallMaterial Enum" :default "NewEnumerator0"))
  (bind _gravityportaleffect (`self.GravityPortalEffect`))
  ;[1 0 0] StateChanged
  (switch `/Game/Blueprints/Enums/E_BallMaterial` BallState
    (:`NewEnumerator0`
      (`ActorComponent.SetComponentTickEnabled` _gravityportaleffect true))
    (:`NewEnumerator1`
      (`ActorComponent.SetComponentTickEnabled` _gravityportaleffect false))))

(event `SaveBallLocation`
  ;[1 1 1] Keep Saving Safe Location
  (bind _bisfalling (`self.IsFalling`))
  (if (not _bisfalling)
    (bind _output_get (set `self.SafeLocation` (`self.K2_GetActorLocation`)))
    (`self.SetSafeLocation` _output_get))
  (`KismetSystemLibrary.Delay` 1.0)
  (`self.SaveBallLocation`))

(event `InputAxis|Turn`
  (params (AxisValue :type "Float (single-precision)"))
  ;[0 0.4235 1] Camera Movement
  (`self.AddControllerYawInput` AxisValue))

(event `InputAxis|Zoom`
  (params (AxisValue :type "Float (single-precision)"))
  ;[0 0.4235 1] Camera Movement
  (`self.SetZoomAmount` AxisValue))

(event `WallRollEvent`
  (params (ObjectRef :type "PrimitiveComponent Object Reference") (bIsOnWall :type Boolean) (Normal :type "Vector Structure"))
  ;[0.1098 0 1] WallRollEvent
  (`PrimitiveComponent.SetEnableGravity` ObjectRef (not bIsOnWall))
  (set `self.bIsOnWall` bIsOnWall)
  (set `self.PlaneNormal` Normal))

(event `self.ReceiveHit`
  (params (MyComp :type "PrimitiveComponent Object Reference") (Other :type "Actor Object Reference") (OtherComp :type "PrimitiveComponent Object Reference") (bSelfMoved :type Boolean) (HitLocation :type "Vector Structure") (HitNormal :type "Vector Structure") (NormalImpulse :type "Vector Structure") (Hit :type "HitResult Structure (by ref)"))
  ;[1 1 1] LookIntoIt
  (set `self.DownForce` HitNormal)
  (`self.UpdatePlayerState` OtherComp))

(event `self.ReceiveTick`
  (params (DeltaSeconds :type "Float (single-precision)"))
  (`self.Lerp Arm Length` DeltaSeconds)
  (switch `/Game/Blueprints/Enums/EPlayerInteractionState` (`self.GroundState`)
    (:`NewEnumerator1`
      ;[1 1 1] Add Force OnWall Grip
      (if (`self.bIsOnWall`)
        (`PrimitiveComponent.AddForce` (`self.Sphere`) (* (`self.DownForce`) -1000.0) "None" true) ; This is to make the player stick to the wall
      ))
    (:`NewEnumerator2`
      ;[1 1 1] Add Force When Slippint
      (bind _returnvalue (`PrimitiveComponent.GetPhysicsLinearVelocity` (`self.Sphere`) "None"))
      (bind (_returnvalue_x _returnvalue_y) (`KismetMathLibrary.BreakVector` (* _returnvalue (`self.SlippingForce`))))
      (`PrimitiveComponent.AddForce` (`self.Sphere`) (`KismetMathLibrary.MakeVector` _returnvalue_x _returnvalue_y) "None" false))))

(event `self.Sphere.OnComponentBeginOverlap`
  (params (OverlappedComponent :type "PrimitiveComponent Object Reference") (OtherActor :type "Actor Object Reference") (OtherComp :type "PrimitiveComponent Object Reference") (OtherBodyIndex :type Integer) (bFromSweep :type Boolean) (SweepResult :type "HitResult Structure (by ref)"))
  (`|ExecutionSequence`
    (:`then_0`
      (cast `/Game/Blueprints/Actors/BP_GravityPortal` OtherActor)
      (`self.SetState` "NewEnumerator0"))
    (:`then_1`
      (`/Engine/EditorBlueprintResources/StandardMacros.IsValid` OtherActor
        (:`Is Valid`
          (if (`self.ActorHasTag` OtherActor "Walkable")
            (if (`|EnumEquality` (`self.EBallState`) "NewEnumerator1")
              (`self.WallRollEvent` (`self.Sphere`) true (`.ImpactNormal` (`GameplayStatics.BreakHitResult` SweepResult))))))))))

(event `self.Sphere.OnComponentEndOverlap`
  (params (OverlappedComponent :type "PrimitiveComponent Object Reference") (OtherActor :type "Actor Object Reference") (OtherComp :type "PrimitiveComponent Object Reference") (OtherBodyIndex :type Integer))
  (if (`self.ActorHasTag` OtherActor "Walkable")
    (`self.WallRollEvent` (`self.Sphere`))))

(fn `CheckHitGround`
  (bind _returnvalue (`SceneComponent.K2_GetComponentLocation` (`self.Sphere`)))
  (bind (_outhit _returnvalue_2) (`KismetSystemLibrary.LineTraceSingle` :`Start` _returnvalue :`End` (+ _returnvalue (* (`KismetMathLibrary.Vector_Down`) (`self.Radui`))) :`TraceChannel` "TraceTypeQuery1" :`DrawDebugType` "ForDuration"))
  (set `self.isGrounded` _returnvalue_2))

(fn `CheckOnWall`
  (locals (`overlap Wall` :type Boolean)))

(fn `ClampSpeed`
  (bind _sphere (`self.Sphere`))
  (bind _returnvalue (`PrimitiveComponent.GetPhysicsLinearVelocity` _sphere "None"))
  (`PrimitiveComponent.SetPhysicsLinearVelocity` _sphere (* (`KismetMathLibrary.Normal` _returnvalue) (`KismetMathLibrary.FMin` (`KismetMathLibrary.VSize` _returnvalue) (`self.MaxSpeed`))) false "None"))

(fn `GetSafeLocation`
  (returns (SafeLocation :type "Vector Structure"))
  (return (`self.SafeLocation`)))

(fn `IsFalling`
  (returns (bIsFalling :type Boolean))
  (return (< (.z (`self.GetVelocity`)) 0.0)))

(fn `Lerp Arm Length`
  (params (`Delta Time` :type "Float (double-precision)"))
  (bind _springarm (`self.SpringArm`))
  (set `SpringArmComponent.TargetArmLength` (`KismetMathLibrary.Lerp` (`SpringArmComponent.TargetArmLength` _springarm) (`self.currentArmDistance`) (* `Delta Time` 4.0)) _springarm))

(fn `Respawn`
  (params (SpawnLocation :type "Vector Structure"))
  (returns (TimesRespawned :type "Float (double-precision)"))
  (locals (TimesSpawned :type "Float (double-precision)"))
  (`self.K2_SetActorLocation` SpawnLocation false true)
  (`PrimitiveComponent.SetAllPhysicsLinearVelocity` (`self.Sphere`) (0.0 0.0 0.0) false)
  (bind _result (`/Engine/EditorBlueprintResources/StandardMacros.IncrementFloat` (`self.Times Respawned`))
    (:`  `
      (return _result))))

(fn `SetLookAtWall`
  (bind _returnvalue (`SceneComponent.GetForwardVector` (`self.Camera`)))
  (bind _returnvalue_2 (`SceneComponent.K2_GetComponentLocation` (`self.Sphere`)))
  (if (`self.bIsOnWall`)
    (bind (_outhit _returnvalue_3) (`KismetSystemLibrary.LineTraceSingle` _returnvalue_2 (+ _returnvalue_2 (* _returnvalue 1000.0) (* _returnvalue (`self.Radui`))) "TraceTypeQuery1"))
    (bind (_bblockinghit _binitialoverlap _time _distance _location _impactpoint _normal _impactnormal _physmat _hitactor) (`GameplayStatics.BreakHitResult` _outhit))
    (`/Engine/EditorBlueprintResources/StandardMacros.IsValid` _hitactor
      (:`Is Valid`
        (if (not (and (`self.ActorHasTag` _hitactor "Walkable") _returnvalue_3))
          (`PrimitiveComponent.SetEnableGravity` (`self.Sphere`) true :!label _label)
          (set `self.bIsOnWall` false)
          (`KismetSystemLibrary.PrintString` "Wall Gravity"))))
    (else
      (goto _label))))

(fn `SetMaterial`
  (returns (index :type Integer))
  (bind _materials (`self.Materials`))
  (bind _currentmat (`self.currentMat`))
  (set `self.currentMat` (mod (`self.currentMat`) (`BlueprintMapLibrary.Map_Length` _materials)))
  (`|ExecutionSequence`
    (:`then_0`
      (bind _values (`BlueprintMapLibrary.Map_Values` _materials))
      (bind _output_get (set `self.EBallState` (`|GetArrayItem` _values _currentmat)))
      (`self.BallStateSwitched` _output_get))
    (:`then_1`
      (bind _keys (`BlueprintMapLibrary.Map_Keys` _materials))
      (`PrimitiveComponent.SetMaterial` (`self.Sphere`) 0 (`|GetArrayItem` _keys _currentmat))
      (return 0))))

(fn `SetState`
  (params (SetState :type "/Game/Blueprints/Enums/EPlayerInteractionState Enum" :default "NewEnumerator0"))
  (bind _sphere (`self.Sphere`))
  (bind _movementspeed (`self.MovementSpeed`))
  (bind _output_get (set `self.GroundState` SetState))
  (switch `/Game/Blueprints/Enums/EPlayerInteractionState` _output_get
    (:`NewEnumerator0`
      (set `self.currentMovementSpeed` _movementspeed)
      (`PrimitiveComponent.SetLinearDamping` _sphere 0.05))
    (:`NewEnumerator1`
      (set `self.currentMovementSpeed` (/ _movementspeed 2.0))
      (`PrimitiveComponent.SetLinearDamping` _sphere 2.0))
    (:`NewEnumerator2`
      (set `self.currentMovementSpeed` 0.0)
      (`PrimitiveComponent.SetLinearDamping` _sphere 0.0))))

(fn `SetZoomAmount`
  (params (value :type "Float (double-precision)"))
  (returns (`Lerp Time Need` :type "Float (double-precision)"))
  (locals (zoomSpeed :type "Float (double-precision)" :default 1000.0) (`Diff Value` :type "Float (double-precision)"))
  (bind _currentarmdistance (`self.currentArmDistance`))
  (bind (_armlimitationdistance_x _armlimitationdistance_y) (`KismetMathLibrary.BreakVector2D` (`self.ArmLimitationDistance`)))
  (bind _returnvalue (`KismetMathLibrary.FClamp` (+ (* value (`local.zoomSpeed`) (`GameplayStatics.GetWorldDeltaSeconds`) -1.0) _currentarmdistance) _armlimitationdistance_x _armlimitationdistance_y))
  (bind _output_get (set `local.Diff Value` (`KismetMathLibrary.Abs` (- _returnvalue _currentarmdistance))))
  (set `self.currentArmDistance` _returnvalue)
  (return _output_get))

(fn `UpdatePlayerState`
  (params (`Collided Comp` :type "PrimitiveComponent Object Reference"))
  (bind _returnvalue (`PrimitiveComponent.GetMaterial` `Collided Comp` 0))
  (bind _eballstate (`self.EBallState`))
  (bind _returnvalue_2 (`MaterialInterface.GetPhysicalMaterial` _returnvalue))
  (`/Engine/EditorBlueprintResources/StandardMacros.IsValid` _returnvalue
    (:`Is Valid`
      (`/Engine/EditorBlueprintResources/StandardMacros.IsValid` _returnvalue_2
        (:`Is Valid`
          (switch `EPhysicalSurface` (`PhysicalMaterial.SurfaceType` _returnvalue_2)
            (:`SurfaceType_Default`
              (`self.SetState` "NewEnumerator0" :!label _label))
            (:`SurfaceType1`
              (switch `/Game/Blueprints/Enums/E_BallMaterial` _eballstate
                (:`NewEnumerator0`
                  (`self.SetState` "NewEnumerator2"))
                (:`NewEnumerator1`
                  (goto _label))))
            (:`SurfaceType2`
              (switch `/Game/Blueprints/Enums/E_BallMaterial` _eballstate
                (:`NewEnumerator0`
                  (goto _label))
                (:`NewEnumerator1`
                  (`self.SetState` "NewEnumerator1"))))))))))

(fn `UserConstructionScript`)