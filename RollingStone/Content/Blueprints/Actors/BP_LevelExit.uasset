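; BP_LevelExit is a level exit trigger that stops the player ball and banks its score.
; When BP_PlayerBall overlaps the Box while CanEndLevel is true, it disables the ball's movement and calls ManageScore.
; ManageScore adds the BPCScoreCounter score to GI_ProgressManager, cached at BeginPlay, then resets the counter.
; The LerpVelocity timeline then eases the ball's physics velocity from its entry value to zero.
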(event `self.ReceiveBeginPlay`
  (bind _asgi_progress_manager (cast `/Game/Blueprints/GI_ProgressManager` (`GameplayStatics.GetGameInstance`)))
  (set `self.GameInstance` _asgi_progress_manager))

(event `self.Box.OnComponentBeginOverlap`
  (params (OverlappedComponent :type "PrimitiveComponent Object Reference") (OtherActor :type "Actor Object Reference") (OtherComp :type "PrimitiveComponent Object Reference") (OtherBodyIndex :type Integer) (bFromSweep :type Boolean) (SweepResult :type "HitResult Structure (by ref)"))
  (bind _asbp_player_ball (cast `/Game/Blueprints/Actors/BP_PlayerBall` OtherActor))
  (if (`self.bCanEndLevel`)
    (set `/Game/Blueprints/Actors/BP_PlayerBall.CanMove` false _asbp_player_ball)
    (`self.ManageScore` _asbp_player_ball)
    (bind _sphere (`/Game/Blueprints/Actors/BP_PlayerBall.Sphere` _asbp_player_ball))
    (set `self.BallVelocityOnEnter` (`SceneComponent.GetComponentVelocity` _sphere))
    (bind (_direction _alpha) (`Timeline|Lerp Velocity`)
      (:`Update`
        (`PrimitiveComponent.SetPhysicsLinearVelocity` _sphere (`KismetMathLibrary.VLerp` (`self.BallVelocityOnEnter`) (0.0 0.0 0.0) _alpha) false "None")))))

(fn `ManageScore`
  (params (PlayerBall :type "/Game/Blueprints/Actors/BP_PlayerBall Object Reference"))
  (bind _gameinstance (`self.GameInstance`))
  (bind _bp_c_scorecounter (`/Game/Blueprints/Actors/BP_PlayerBall.BP_C_ScoreCounter` PlayerBall))
  (`/Engine/EditorBlueprintResources/StandardMacros.IsValid` _gameinstance
    (:`Is Valid`
      (`/Game/Blueprints/GI_ProgressManager.AddScore` _gameinstance (`/Game/Blueprints/Components/BP_C_ScoreCounter.GetScore` _bp_c_scorecounter))
      (`/Game/Blueprints/Components/BP_C_ScoreCounter.ResetScore` _bp_c_scorecounter))))

(fn `UserConstructionScript`)